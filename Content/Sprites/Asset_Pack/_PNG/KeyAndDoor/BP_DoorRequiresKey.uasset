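; Door actor for a Paper2D game that either plays a locked sound or sends the player to the Cave level.
; On overlap by a PaperCharacter it branches on its own HasKey flag, where true plays the locked sound.
; When false, it plays the open sound, runs a WB_Fade widget animation, waits briefly, opens the level and then sets HasKey to false.
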(event `self.ReceiveActorBeginOverlap`
  (params (OtherActor :type "Actor Object Reference"))
  (cast `PaperCharacter` OtherActor)
  (if (`self.hasKey`)
    (`GameplayStatics.PlaySound2D` "/Game/Sprites/Asset_Pack/_PNG/KeyAndDoor/Sound_LockedDoor.Sound_LockedDoor" 1.0 1.0 0.0 null null)
    (else
      (`GameplayStatics.PlaySound2D` "/Game/Sprites/Asset_Pack/_PNG/KeyAndDoor/openDoor.openDoor" 1.0 1.0 0.0 null null)
      (bind _returnvalue (`|CreateWidget` "/Game/Sprites/Asset_Pack/_PNG/KeyAndDoor/WB_Fade.WB_Fade_C"))
      (`UserWidget.AddToViewport` _returnvalue 0)
      (`/Game/Sprites/Asset_Pack/_PNG/KeyAndDoor/WB_Fade.Fade Anim` _returnvalue)
      (`KismetSystemLibrary.Delay` 0.5)
      (`GameplayStatics.OpenLevel` "Cave")
      (set `self.hasKey` false))))

(fn `UserConstructionScript`)